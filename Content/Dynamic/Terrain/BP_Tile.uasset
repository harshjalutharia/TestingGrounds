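; Terrain tile for an infinite terrain mode that, on BeginPlay, starts locked and populates itself with props, rocks and AI characters.
; The player entering LockingVolume turns the red Barrier green and non-colliding; leaving relocks it and reports a conquered tile to BP_InfiniteTerrainGameMode.
; Leaving DeleteTrigger has the game mode spawn a tile, then destroys this one.
; An Arrow component supplies the tile's attach transform.
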(event OnComponentBeginOverlap(LockingVolume)
  (params (OverlappedComponent :type Primitive%20Component%20Object%20Reference) (OtherActor :type Actor%20Object%20Reference) (OtherComp :type Primitive%20Component%20Object%20Reference) (OtherBodyIndex :type Integer) (bFromSweep :type Boolean) (SweepResult :type Hit%20Result%20Structure%20%28by%20ref%29))
  (Utilities|IsPlayerActor OtherActor)
  (CallFunction|Unlock))

(event OnComponentEndOverlap(LockingVolume)
  (params (OverlappedComponent :type Primitive%20Component%20Object%20Reference) (OtherActor :type Actor%20Object%20Reference) (OtherComp :type Primitive%20Component%20Object%20Reference) (OtherBodyIndex :type Integer))
  (Utilities|IsPlayerActor OtherActor)
  (CallFunction|Lock)
  (bind _asbp_infinite_terrain_game_mode (Utilities|Casting|CastToBP_InfiniteTerrainGameMode (Game|GetGameMode)))
  (Default|NewTileConquered _asbp_infinite_terrain_game_mode))

(event OnComponentEndOverlap(DeleteTrigger)
  (params (OverlappedComponent :type Primitive%20Component%20Object%20Reference) (OtherActor :type Actor%20Object%20Reference) (OtherComp :type Primitive%20Component%20Object%20Reference) (OtherBodyIndex :type Integer))
  (Utilities|IsPlayerActor OtherActor)
  (bind _asbp_infinite_terrain_game_mode (Utilities|Casting|CastToBP_InfiniteTerrainGameMode (Game|GetGameMode)))
  (Default|SpawnTile _asbp_infinite_terrain_game_mode)
  (Actor|DestroyActor))

(event EventBeginPlay
  (CallFunction|Lock)
  (Class|Tile|PlaceActors "/Game/Dynamic/Terrain/Props/BP_Container.BP_Container_C" 1 3 425.0 1.0 1.0)
  (Class|Tile|PlaceActors "/Game/Dynamic/Terrain/Props/BP_Box.BP_Box_C" 2 4 1e+02 1.0 1.0)
  (Class|Tile|PlaceActors "/Game/Dynamic/Terrain/Props/BP_Canister.BP_Canister_C" 1 7 5e+01 1.0 1.0)
  (Class|Tile|PlaceActors "/Game/Dynamic/Terrain/Props/BP_Rock1.BP_Rock1_C" 1 4 1.5e+02 1.0 5.0)
  (Class|Tile|PlaceActors "/Game/Dynamic/Terrain/Props/BP_Rock2.BP_Rock2_C" 1 4 275.0 1.0 5.0)
  (Class|Tile|PlaceActors "/Game/Dynamic/Terrain/Props/BP_Rock3.BP_Rock3_C" 1 4 2.5e+02 1.0 5.0)
  (Class|Tile|PlaceActors "/Game/Dynamic/Terrain/Props/BP_Sandbags.BP_Sandbags_C" 1 3 2e+02 1.0 1.0)
  (Class|Tile|PlaceAIPawns "/Game/Dynamic/Character/Behaviour/BP_Character.BP_Character_C" 2 4 1e+02))

(fn ConstructionScript)

(fn GetAttachLocation
  (return (Transformation|GetWorldTransform (Variables|Default|GetArrow))))

(fn Unlock
  (bind _barrier (Variables|Default|GetBarrier))
  (Collision|SetCollisionEnabled _barrier "NoCollision")
  (Rendering|Material|SetMaterial _barrier 0 "/Game/Dynamic/Terrain/MI_Barrier_Green.MI_Barrier_Green"))

(fn Lock
  (bind _barrier (Variables|Default|GetBarrier))
  (Collision|SetCollisionEnabled _barrier "QueryAndPhysics")
  (Rendering|Material|SetMaterial _barrier 0 "/Game/Dynamic/Terrain/MI_Barrier_Red.MI_Barrier_Red"))